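; Duel manager for a samurai quick-draw between the player and an NPC, driven by an Intro, Wait, Draw, Finish phase state.
; Tick waits out the intro, then a random delay before broadcasting the draw event, showing the exclamation cue and starting a restart timer.
; Functions defeat the loser and hide the cue, mark the duel finished, or reset both samurai and the phase.
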(event EventBeginPlay
  (bind _returnvalue (Actor|GetActorOfClass "/Game/Blueprints/BP_Exclamaçao.BP_Exclamaçao_C"))
  (Variables|Default|SetExclamationRef _returnvalue)
  (bind _returnvalue_2 (Actor|GetActorOfClass "/Game/Blueprints/BP_Samurai_Player.BP_Samurai_Player_C"))
  (Variables|Default|SetSamurai%20Player _returnvalue_2)
  (bind _returnvalue_3 (Actor|GetActorOfClass "/Game/Blueprints/BP_Samurai_NPC.BP_Samurai_NPC_C"))
  (Variables|Default|SetSamuraiNPC _returnvalue_3))

(event EventTick
  (params (DeltaSeconds :type Float%20%28single-precision%29))
  (Variables|Default|SetElapsedTime (+ DeltaSeconds (Variables|Default|GetElapsedTime)))
  (switch Utilities|FlowControl|Switch|SwitchonE_Phase (Variables|Default|GetPhase)
    (:NewEnumerator0
      (if (>= (Variables|Default|GetElapsedTime) (Variables|Default|GetRoundStartTime))
        (Variables|Default|SetPhase "NewEnumerator1")
        (Utilities|FlowControl|Delay (Math|Random|RandomFloatinRange (Variables|Default|GetMin%20Draw%20Delay) (Variables|Default|GetMax%20Draw%20%20Delay)))
        (Variables|Default|SetPhase "NewEnumerator2")
        (Default|CallDrawEventStarted)
        (Utilities|IsValid (Variables|Default|GetExclamationRef)
          (:Is%20Valid
            (Default|SetVisibilit (Variables|Default|GetExclamationRef) true)
            (Utilities|Time|SetTimerbyEvent (EventDispatchers|CreateEvent :!event Reset) (Variables|Default|GetRestard%20Delay))))))))

(fn ConstructionScript)

(fn SetGameFinish
  (Variables|Default|SetPhase "NewEnumerator3"))

(fn AttackSuccssfully
  (params (is%20Player :type Boolean))
  (if is%20Player
    (Default|Defeated (Variables|Default|GetSamuraiNPC))
    (else
      (Default|Defeated (Variables|Default|GetSamurai%20Player))))
  (Utilities|IsValid (Variables|Default|GetExclamationRef)
    (:Is%20Valid
      (Default|SetVisibilit (Variables|Default|GetExclamationRef) false))))

(fn Reset
  (bind _samurai_player (Variables|Default|GetSamurai%20Player))
  (Variables|Default|SetPhase "NewEnumerator0")
  (Variables|Default|SetElapsedTime 0.0)
  (Default|Reset _samurai_player)
  (Default|Reset (Variables|Default|GetSamuraiNPC))
  (Default|SetCrossVisibilit _samurai_player false))