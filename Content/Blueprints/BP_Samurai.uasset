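; BP_Samurai is a duelist in a quick-draw duel, driven by the Gm_Duel game mode's phase.
; Timelines slide its sprite in on BeginPlay and Reset.
; Attack shows a cross during Wait; during Draw it ends the round and lunges, with a timeline event swapping sprites and reporting success with whether it is player-controlled.
; Defeated shows the losing sprite and cross, while Reset restores idle without hiding the cross.
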(event Custom|Slideln
  (Components|Timeline|SetPlayRate (Variables|Default|GetSlidelnAnim) 2.0)
  (bind _slideranim (Timeline|SlidelnAnim PlayFromStart)
    (:Update
      (Transformation|SetRelativeLocation (Variables|Default|GetPaperSprite) (Math|Vector|Lerp(Vector) (Variables|Default|GetSlider%20Start%20Pos) (Variables|Default|GetSprite%20Defoult%20Pos) _slideranim) false false))))

(event Custom|Attack
  (if (not (Variables|Default|GetPressed%20Draw))
    (switch Utilities|FlowControl|Switch|SwitchonE_Phase (Variables|/Game/Blueprints/Gm_Duel.Gm_Duel_C|GetPhase (Variables|Default|GetGame%20Mode))
      (:NewEnumerator1
        (CallFunction|SetCrossVisibilit true)
        (Variables|Default|SetPressed%20Draw false))
      (:NewEnumerator2
        (Variables|Default|SetPressed%20Draw true)
        (Default|SetGameFinish (Variables|Default|GetGame%20Mode))
        (CallFunction|SetSprite "/Game/Paper_Assets/Tanuki/T_Tanuki_Attack_Sprite.T_Tanuki_Attack_Sprite")
        (Components|Timeline|SetPlayRate (Variables|Default|GetAttackAnim) 8.0)
        (bind _alpha (Timeline|AttackAnim PlayFromStart)
          (:Update
            (Transformation|SetRelativeLocation (Variables|Default|GetPaperSprite) (Math|Vector|Lerp(Vector) (Variables|Default|GetSprite%20Defoult%20Pos) (Variables|/Script/Engine.SceneComponent|GetRelativeLocation (Variables|Default|GetAttackPos)) _alpha) false false))
          (:SwitcSprite
            (Audio|SpawnSound2D "/Game/Sound/Espada/knife-slice-41231.knife-slice-41231" 1.0 1.0 0.0 0)
            (CallFunction|SetSprite (Variables|Default|GetAttack%20Spride))
            (Default|AttackSuccssfully (Variables|Default|GetGame%20Mode) (Pawn|IsPlayerControlled))
            (Audio|SpawnSound2D (Variables|Default|GetGrito) 7.0 1.0 0.0 0)))))))

(event Custom|Defeated
  (CallFunction|SetSprite (Variables|Default|GetDefeated%20Spride))
  (CallFunction|SetCrossVisibilit true))

(event EventBeginPlay
  (Audio|SpawnSound2D "/Game/Sound/swingbee-157396.swingbee-157396" 0.5 1.0 0.0 0)
  (bind _asgm_duel (Utilities|Casting|CastToGm_Duel (Game|GetGameMode)))
  (Variables|Default|SetGame%20Mode _asgm_duel)
  (Variables|Default|SetSprite%20Defoult%20Pos (Variables|/Script/Engine.SceneComponent|GetRelativeLocation (Variables|Default|GetPaperSprite)))
  (CallFunction|Slideln)
  (CallFunction|SetCrossVisibilit false))

(event Collision|EventActorBeginOverlap
  (params (OtherActor :type Actor%20Object%20Reference)))

(event EventTick
  (params (DeltaSeconds :type Float%20%28single-precision%29)))

(fn ConstructionScript)

(fn SetCrossVisibilit
  (params (bNewVisibility :type Boolean))
  (Rendering|SetVisibility (Variables|Default|GetCrosss) bNewVisibility false))

(fn SetSprite
  (params (NewSprite :type Paper%20Sprite%20Object%20Reference))
  (Rendering|Components|Sprite|SetSprite (Variables|Default|GetPaperSprite) NewSprite))

(fn Reset
  (CallFunction|SetSprite (Variables|Default|GetIdleSprit))
  (Variables|Default|SetPressed%20Draw false)
  (CallFunction|Slideln))